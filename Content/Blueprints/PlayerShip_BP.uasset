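; Player ship pawn Blueprint that handles the game's end screens and pause menu.
; Each Tick it casts the player pawn to its own class and polls the level value and game-over getters, showing the champions widget at level six or the game-over widget when flagged.
; The MenuPausa input action opens the pause menu.
; All three paths pause the game, switch to UI-only input and show the cursor.
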(event Collision|EventActorBeginOverlap
  (params (OtherActor :type Actor%20Object%20Reference)))

(event EventTick
  (params (DeltaSeconds :type Float%20%28single-precision%29))
  (bind _returnvalue (Game|GetPlayerController 0))
  (bind _returnvalue_2 (Game|GetPlayerController 0))
  (Utilities|FlowControl|Sequence
    (:then_0
      (bind _asplayer_ship_bp (Utilities|Casting|CastToPlayerShip_BP (Game|Player|GetPlayerPawn 0)))
      (bind _returnvalue_3 (Class|PlayerShip|GetLevelValue _asplayer_ship_bp))
      (switch int _returnvalue_3
        (:6
          (bind _returnvalue_4 (UserInterface|CreateWidget "/Game/Blueprints/Widgets/WG_Champions.WG_Champions_C" _returnvalue))
          (UserInterface|Viewport|AddtoViewport _returnvalue_4 0)
          (Game|SetGamePaused true)
          (Input|SetInputModeUIOnly _returnvalue _returnvalue_4 "DoNotLock")
          (Variables|/Script/Engine.PlayerController|SetbShowMouseCursor _returnvalue true))))
    (:then_1
      (bind _asplayer_ship_bp_2 (Utilities|Casting|CastToPlayerShip_BP (Game|Player|GetPlayerPawn 0)))
      (bind _returnvalue_5 (Class|PlayerShip|GetGameOver _asplayer_ship_bp_2))
      (switch int _returnvalue_5
        (:1
          (bind _returnvalue_6 (UserInterface|CreateWidget "/Game/Blueprints/Widgets/WG_GameOver.WG_GameOver_C" _returnvalue_2))
          (UserInterface|Viewport|AddtoViewport _returnvalue_6 0)
          (Game|SetGamePaused true)
          (Input|SetInputModeUIOnly _returnvalue_2 _returnvalue_6 "DoNotLock")
          (Variables|/Script/Engine.PlayerController|SetbShowMouseCursor _returnvalue_2 true))))))

(event EventBeginPlay)

(event Input|ActionEvents|InputActionMenuPausa
  (params (Key :type Key%20Structure :default "None"))
  (bind _returnvalue (Game|GetPlayerController 0))
  ;[1 1 1] Menu pausa
  (:Pressed
    (Game|SetGamePaused true)
    (bind _returnvalue_2 (UserInterface|CreateWidget "/Game/Menus/PauseMenu/WG_PauseMenu.WG_PauseMenu_C" _returnvalue))
    (UserInterface|Viewport|AddtoViewport _returnvalue_2 0)
    (Input|SetInputModeUIOnly _returnvalue _returnvalue_2 "DoNotLock")
    (Variables|/Script/Engine.PlayerController|SetbShowMouseCursor _returnvalue true)))

(fn ConstructionScript)